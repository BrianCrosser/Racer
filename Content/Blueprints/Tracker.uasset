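; Race tracker that runs a lap-based checkpoint race, pushing lap count, medal times and default bests to MyPlayerController at BeginPlay.
; It numbers the Checkpoints array, binds each one's cleared event, starts level music and activates the first checkpoint.
; Each clear plays a sound, updates the respawn transform and reveals the next trigger.
; The final checkpoint updates the lap and either loops to the first or completes the race, triggering the controller's Restart.
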(event Custom|ApplySettings
  (bind _controllerreference (Variables|Default|GetControllerReference))
  (Variables|/Game/Blueprints/MyPlayerController.MyPlayerController_C|SetMaxLaps _controllerreference (Variables|CustomSettings|GetMaxLaps))
  (CallFunction|UpdateTimes)
  (Default|StartGameSetup _controllerreference))

(event Custom|CheckpointCleared
  (params (NextCheckpoint :type Integer))
  (bind _controllerreference (Variables|Default|GetControllerReference))
  (CallFunction|LapCheck NextCheckpoint)
  (Audio|Components|Audio|Play (Variables|/Script/Engine.AmbientSound|GetAudioComponent (Variables|CustomSettings|GetCheckpointSoundFX)) 0.0)
  (if (Variables|/Game/Blueprints/MyPlayerController.MyPlayerController_C|GetRaceComplete _controllerreference)
    (Default|Restart _controllerreference)))

(event Custom|StartSequence
  (bind _checkpoints (Variables|Checkpoints|GetCheckpoints))
  (for (_array_element _array_index) (Variables|Checkpoints|GetCheckpoints)
    (Variables|/Game/Blueprints/Checkpoint.Checkpoint_C|SetCheckpointNumber _array_element (+ _array_index 1))
    (Variables|Default|SetTotalCheckpoints (Utilities|Array|Length _checkpoints))
    (CallFunction|ActivateCheckpoint (Utilities|Array|Get(acopy) _checkpoints))
    (for _array_element_2 (Variables|Checkpoints|GetCheckpoints)
      (EventDispatchers|AssignCheckpointCleared _array_element_2 (delegate Custom|CheckpointCleared))
      (Audio|Components|Audio|Play (Variables|/Script/Engine.AmbientSound|GetAudioComponent (Variables|CustomSettings|GetLevelMusic)) 0.0))))

(event EventBeginPlay
  (bind _asmy_player_controller (Utilities|Casting|CastToMyPlayerController (Game|GetPlayerController 0)))
  (Variables|Default|SetControllerReference _asmy_player_controller)
  (CallFunction|ApplySettings)
  (CallFunction|StartSequence))

(fn ConstructionScript)

(fn UpdateTimes
  (bind _controllerreference (Variables|Default|GetControllerReference))
  (Variables|/Game/Blueprints/MyPlayerController.MyPlayerController_C|SetGoldTime _controllerreference (Variables|CustomSettings|GetGoldTime))
  (Variables|/Game/Blueprints/MyPlayerController.MyPlayerController_C|SetSilverTime _controllerreference (Variables|CustomSettings|GetSilverTime))
  (Variables|/Game/Blueprints/MyPlayerController.MyPlayerController_C|SetBronzeTime _controllerreference (Variables|CustomSettings|GetBronzeTime))
  (Variables|/Game/Blueprints/MyPlayerController.MyPlayerController_C|SetDefaultBestLapTime _controllerreference (Variables|CustomSettings|GetDefaultBestLap))
  (Variables|/Game/Blueprints/MyPlayerController.MyPlayerController_C|SetBestRaceTime _controllerreference (Variables|CustomSettings|GetDefaultBestTime)))

(fn LapCheck
  (params (Checkpoint :type Integer))
  (bind _output_get (LocalVariables|SetLocalCheckpoint Checkpoint))
  (if (== _output_get (Variables|Default|GetTotalCheckpoints))
    (bind _isracecompleted (CallFunction|RaceCompleteCheck))
    (if _isracecompleted
      _
      (else
        (CallFunction|ActivateCheckpoint (Utilities|Array|Get(acopy) (Variables|Checkpoints|GetCheckpoints)))))
    (Default|UpdateLap (Variables|Default|GetControllerReference))
    (else
      (CallFunction|ActivateCheckpoint (Utilities|Array|Get(acopy) (Variables|Checkpoints|GetCheckpoints) (LocalVariables|GetLocalCheckpoint)))))
  (Variables|/Game/Blueprints/MyPlayerController.MyPlayerController_C|SetRespawnLocation (Variables|Default|GetControllerReference) (Transformation|GetActorTransform (Utilities|Array|Get(acopy) (Variables|Checkpoints|GetCheckpoints) (- (LocalVariables|GetLocalCheckpoint) 1)))))

(fn ActivateCheckpoint
  (params (NextCheckpoint :type Checkpoint%20Object%20Reference))
  (bind _trigger (Variables|/Game/Blueprints/Checkpoint.Checkpoint_C|GetTrigger NextCheckpoint))
  (Development|SetHiddeninGame _trigger false false)
  (Variables|/Script/Engine.PrimitiveComponent|SetbGenerateOverlapEvents _trigger true))

(fn RaceCompleteCheck
  (bind _controllerreference (Variables|Default|GetControllerReference))
  (bind _controllerreference_2 (Variables|Default|GetControllerReference))
  (if (>= (Variables|/Game/Blueprints/MyPlayerController.MyPlayerController_C|GetActualLap _controllerreference) (Variables|/Game/Blueprints/MyPlayerController.MyPlayerController_C|GetMaxLaps _controllerreference))
    (bind _output_get (Variables|/Game/Blueprints/MyPlayerController.MyPlayerController_C|SetRaceComplete _controllerreference_2 true))
    (LocalVariables|SetLocalComplete _output_get)
    (else
      (bind _output_get_2 (Variables|/Game/Blueprints/MyPlayerController.MyPlayerController_C|SetRaceComplete _controllerreference_2 false))
      (LocalVariables|SetLocalComplete _output_get_2)))
  (return (LocalVariables|GetLocalComplete)))