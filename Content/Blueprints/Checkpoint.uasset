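; Checkpoint Blueprint that detects a vehicle passing through it in the intended direction.
; When a VehicleBlueprint leaves the Trigger, the dot product of its velocity and the Arrow's forward vector must be positive.
; A valid pass fires the CheckpointCleared dispatcher with the checkpoint's number and hides the trigger and particle system in game.
; It also sets overlap events on the Trigger to enabled, so overlap detection stays on.
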(event OnComponentEndOverlap(Trigger)
  (params (OtherActor :type Actor%20Object%20Reference) (OtherComp :type Primitive%20Component%20Object%20Reference) (OtherBodyIndex :type Integer))
  (bind _trigger (Variables|Default|GetTrigger))
  (bind _asvehicle_blueprint (Utilities|Casting|CastToVehicleBlueprint OtherActor))
  (if (> (Math|Vector|DotProduct (Transformation|GetVelocity _asvehicle_blueprint) (Math|Rotator|GetRotationXVector (Transformation|GetWorldRotation (Variables|Default|GetArrow)))) 0.0)
    (Default|CallCheckpointCleared (Variables|Default|GetCheckpointNumber))
    (Development|SetHiddeninGame _trigger true false)
    (Variables|/Script/Engine.PrimitiveComponent|SetbGenerateOverlapEvents _trigger true)))

(fn ConstructionScript)