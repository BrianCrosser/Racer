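; Player controller for a lap-based racing game that runs the HUD, click-started countdown, race and lap timing, vehicle respawn and level restart.
; Timelines drive race and lap clocks, with race time progressively hiding missed gold, silver and bronze goals.
; Lap updates check for best lap and, on completion, best race time, saving records to a SaveGame slot.
; R resets records before the race starts; P prints them.
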(event Custom|StartGameSetup
  (CallFunction|SaveGameCheck)
  (CallFunction|InitText))

(event Custom|StopLapTime
  (bind _time (Timeline|LapTime Stop)
    (:Update
      (Variables|ValueVariables|SetActualLapTime _time))))

(event Custom|UpdateLap
  (if (Variables|Default|GetRaceComplete)
    _
    (else
      (bind _output_get (Variables|ValueVariables|SetActualLap (+ (Variables|ValueVariables|GetActualLap) 1)))
      (Variables|TextVariables|SetCurrentLapText (Utilities|Text|ToText(Integer) _output_get))))
  (CallFunction|LapTimeCheck))

(event Custom|RespawnVehicle
  (bind _returnvalue (Game|SpawnActorfromClass "/Game/VehicleAdvBP/Blueprints/VehicleBlueprint.VehicleBlueprint_C" (Variables|Default|GetRespawnLocation) "Undefined" 0 0))
  (Pawn|Possess _returnvalue))

(event Custom|StartRaceTime
  (bind _time (Timeline|GameTime Play)
    (:Update
      (bind _output_get (Variables|ValueVariables|SetActualRaceTime _time))
      (Variables|TextVariables|SetRaceTimeText (Utilities|TimetoText _output_get))
      (CallFunction|UpdateGoals))))

(event Custom|StopRaceTime
  (bind _time (Timeline|GameTime Stop)
    (:Update
      (bind _output_get (Variables|ValueVariables|SetActualRaceTime _time))
      (Variables|TextVariables|SetRaceTimeText (Utilities|TimetoText _output_get))
      (CallFunction|UpdateGoals))))

(event Custom|Restart
  (Variables|Default|SetRaceStart false)
  (Utilities|FlowControl|Delay 6.0)
  (Development|ExecuteConsoleCommand "Restartlevel"))

(event Custom|StartLapTime
  (bind _time (Timeline|LapTime PlayFromStart)
    (:Update
      (Variables|ValueVariables|SetActualLapTime _time))))

(event EventBeginPlay
  (bind _returnvalue (UserInterface|CreateWidget "/Game/Blueprints/UI/HUD.HUD_C"))
  (bind _output_get (Variables|Default|SetHUDReference _returnvalue))
  (UserInterface|Viewport|AddtoViewport _output_get 0)
  (bind _asvehicle_blueprint (Utilities|Casting|CastToVehicleBlueprint (Game|Player|GetPlayerPawn 0)))
  (Variables|Default|SetVehicleReference _asvehicle_blueprint))

(event Input|KeyboardEvents|R
  (params (Key :type Key%20Structure :default "AnyKey"))
  (:Pressed
    (if (not (Variables|Default|GetRaceStart))
      (Variables|ValueVariables|SetBestLapTime (Variables|ValueVariables|GetDefaultBestLapTime))
      (Variables|ValueVariables|SetBestRaceTime (Variables|ValueVariables|GetDefaultBestRaceTime))
      (CallFunction|SavetheGame)
      (CallFunction|InitText))))

(event Input|KeyboardEvents|P
  (params (Key :type Key%20Structure :default "AnyKey"))
  (:Pressed
    (Variables|TextVariables|SetBestLapText (Utilities|TimetoText (Variables|ValueVariables|GetBestLapTime)))
    (Variables|TextVariables|SetBestTimeText (Utilities|TimetoText (Variables|ValueVariables|GetBestRaceTime)))
    (Development|PrintText (Variables|TextVariables|GetBestLapText))
    (Development|PrintText (Variables|TextVariables|GetBestTimeText))))

(event Input|MouseEvents|LeftMouseButton
  (params (Key :type Key%20Structure :default "AnyKey"))
  (bind _hudreference (Variables|Default|GetHUDReference))
  (bind _hudreference_2 (Variables|Default|GetHUDReference))
  (:Pressed
    (Utilities|FlowControl|DoOnce false
      (:Completed
        (Variables|/Game/Blueprints/UI/HUD.HUD_C|SetSplashScreenVisible _hudreference "Hidden")
        (Variables|/Game/Blueprints/UI/HUD.HUD_C|SetCountDownVisible _hudreference "Visible")
        (Utilities|FlowControl|Delay 2.5)
        (Variables|TextVariables|SetReadyText "2")
        (Utilities|FlowControl|Delay 1.0)
        (Variables|TextVariables|SetReadyText "1")
        (Utilities|FlowControl|Delay 1.0)
        (Variables|TextVariables|SetReadyText "GO!")
        (Utilities|FlowControl|Delay 1.0)
        (Variables|/Game/Blueprints/UI/HUD.HUD_C|SetCountDownVisible _hudreference_2 "Hidden")
        (Variables|/Game/Blueprints/UI/HUD.HUD_C|SetGameHUDVisible _hudreference_2 "Visible")
        (Variables|Default|SetRaceStart true)
        (CallFunction|StartRaceTime)
        (CallFunction|StartLapTime)))))

(fn ConstructionScript)

(fn InitText
  (Variables|TextVariables|SetCurrentLapText (Utilities|Text|ToText(Integer) (Variables|ValueVariables|GetActualLap)))
  (Variables|TextVariables|SetMaxLapText (Utilities|Text|ToText(Integer) (Variables|ValueVariables|GetMaxLaps)))
  (Variables|TextVariables|SetGoldTimeText (Utilities|TimetoText (Variables|ValueVariables|GetGoldTime)))
  (Variables|TextVariables|SetSilverTimeText (Utilities|TimetoText (Variables|ValueVariables|GetSilverTime)))
  (Variables|TextVariables|SetBronzeTimeText (Utilities|TimetoText (Variables|ValueVariables|GetBronzeTime)))
  (Variables|TextVariables|SetBestLapText (Utilities|TimetoText (Variables|ValueVariables|GetBestLapTime)))
  (Variables|TextVariables|SetBestTimeText (Utilities|TimetoText (Variables|ValueVariables|GetBestRaceTime))))

(fn SaveGameCheck
  (bind _returnvalue (SaveGame|DoesSaveGameExist (Variables|Default|GetSaveSlot)))
  (if _returnvalue
    (CallFunction|LoadtheGame)
    (else
      (Variables|ValueVariables|SetBestLapTime (Variables|ValueVariables|GetDefaultBestLapTime))
      (Variables|ValueVariables|SetBestRaceTime (Variables|ValueVariables|GetDefaultBestRaceTime))
      (CallFunction|SavetheGame))))

(fn SavetheGame
  (bind _returnvalue (SaveGame|CreateSaveGameObject "/Game/Blueprints/MySaveGame.MySaveGame_C"))
  (bind _output_get (Variables|Default|SetSaveGameReference _returnvalue))
  (bind _asmy_save_game (Utilities|Casting|CastToMySaveGame _output_get))
  (Variables|/Game/Blueprints/MySaveGame.MySaveGame_C|SetSavedBestLap _asmy_save_game (Variables|ValueVariables|GetBestLapTime))
  (Variables|/Game/Blueprints/MySaveGame.MySaveGame_C|SetSavedBestTime _asmy_save_game (Variables|ValueVariables|GetBestRaceTime))
  (SaveGame|SaveGametoSlot (Variables|Default|GetSaveGameReference) (Variables|Default|GetSaveSlot)))

(fn LoadtheGame
  (bind _returnvalue (SaveGame|LoadGamefromSlot (Variables|Default|GetSaveSlot)))
  (bind _asmy_save_game (Utilities|Casting|CastToMySaveGame _returnvalue))
  (Variables|ValueVariables|SetBestLapTime (Variables|/Game/Blueprints/MySaveGame.MySaveGame_C|GetSavedBestLap _asmy_save_game))
  (Variables|ValueVariables|SetBestRaceTime (Variables|/Game/Blueprints/MySaveGame.MySaveGame_C|GetSavedBestTime _asmy_save_game)))

(fn LapTimeCheck
  (CallFunction|StopLapTime)
  (if (<= (Variables|ValueVariables|GetActualLapTime) (Variables|ValueVariables|GetBestLapTime))
    (bind _output_get (Variables|ValueVariables|SetBestLapTime (Variables|ValueVariables|GetActualLapTime)))
    (bind _output_get_2 (Variables|TextVariables|SetBestLapText (Utilities|TimetoText _output_get)))
    (CallFunction|SavetheGame)
    (Development|PrintText _output_get_2)
    (Variables|ValueVariables|SetActualLapTime 0.0)
    (else
      (Variables|ValueVariables|SetActualLapTime 0.0)))
  (if (Variables|Default|GetRaceComplete)
    (CallFunction|RaceTimeCheck)
    (else
      (CallFunction|StartLapTime))))

(fn RaceTimeCheck
  (if (<= (Variables|ValueVariables|GetActualRaceTime) (Variables|ValueVariables|GetBestRaceTime))
    (bind _output_get (Variables|ValueVariables|SetBestRaceTime (Variables|ValueVariables|GetActualRaceTime)))
    (bind _output_get_2 (Variables|TextVariables|SetBestTimeText (Utilities|TimetoText _output_get)))
    (Development|PrintText _output_get_2)
    (CallFunction|SavetheGame)))

(fn UpdateGoals
  (if (not (<= (Variables|ValueVariables|GetActualRaceTime) (Variables|ValueVariables|GetGoldTime)))
    (Utilities|FlowControl|Sequence
      (:then_0
        (Utilities|FlowControl|DoOnce false
          (:Completed
            (Variables|/Game/Blueprints/UI/HUD.HUD_C|SetGoldTimeVisible (Variables|Default|GetHUDReference) "Hidden"))))
      (:then_1
        (if (not (<= (Variables|ValueVariables|GetActualRaceTime) (Variables|ValueVariables|GetSilverTime)))
          (Utilities|FlowControl|Sequence
            (:then_0
              (Utilities|FlowControl|DoOnce false
                (:Completed
                  (Variables|/Game/Blueprints/UI/HUD.HUD_C|SetSilverTimeVisible (Variables|Default|GetHUDReference) "Hidden"))))
            (:then_1
              (if (not (<= (Variables|ValueVariables|GetActualRaceTime) (Variables|ValueVariables|GetBronzeTime)))
                (Utilities|FlowControl|DoOnce false
                  (:Completed
                    (Variables|/Game/Blueprints/UI/HUD.HUD_C|SetBronzeTimeVisible (Variables|Default|GetHUDReference) "Hidden")))))))))))